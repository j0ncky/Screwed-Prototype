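; Player screw character that switches between physics-driven rolling and upright walking by swapping Enhanced Input mapping contexts, hitbox rotation and physics simulation.
; Rolling adds angular velocity to ParentHitbox and turns by yaw scaled to spin speed, while Tick clamps or damps velocities.
; Walking uses movement input for forward only, with a Timeline bounce on the cylinder.
; Tick also keeps the capsule on the hitbox, taking yaw from the spring-arm camera.
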(event `self.ReceiveTick`
  (params (DeltaSeconds :type "Float (single-precision)"))
  (bind (_returnvalue_roll _returnvalue_pitch _returnvalue_yaw) (`KismetMathLibrary.BreakRotator` (`SceneComponent.K2_GetComponentRotation` (`self.SpringArm`))))
  (bind (_returnvalue_roll_2 _returnvalue_pitch_2) (`KismetMathLibrary.BreakRotator` (`SceneComponent.K2_GetComponentRotation` (`self.CapsuleComponent`))))
  (bind _returnvalue (`PrimitiveComponent.GetPhysicsAngularVelocityInRadians` (`self.ParentHitbox`) "None"))
  (set `self.Delta Seconds` DeltaSeconds) ; Initialize Delta Time
  (`SceneComponent.K2_SetWorldLocation` (`self.CapsuleComponent`) (`SceneComponent.K2_GetComponentLocation` (`self.ParentHitbox`)) false false) ; Update Scene Root to location of Capsule
  (`SceneComponent.K2_SetWorldRotation` (`self.CapsuleComponent`) (`KismetMathLibrary.MakeRotator` _returnvalue_roll_2 _returnvalue_pitch_2 _returnvalue_yaw) false false) ; Update Scene Root to rotation of spring arm (camera)
  (`|ExecutionSequence`
    (:`then_0`
      (if (not (`self.bIsWalking`))
        ;[0.15 0.04753 0.09027 0.5] Limits max speed, decreases speed when not moving
        (bind _returnvalue_2 (`PrimitiveComponent.GetPhysicsLinearVelocity` (`self.ParentHitbox`) "None"))
        (if (`self.bIsRolling`)
          (`PrimitiveComponent.SetPhysicsLinearVelocity` (`self.ParentHitbox`) (`KismetMathLibrary.ClampVectorSize` _returnvalue_2 -400.0 400.0) false "None")
          ;[0.3906 0.1221 0.3397 0.5] Limits angular velocity
          (`PrimitiveComponent.SetPhysicsAngularVelocityInRadians` (`self.ParentHitbox`) (`KismetMathLibrary.ClampVectorSize` _returnvalue -16.0 16.0) false "None")
          (else
            (`PrimitiveComponent.SetPhysicsLinearVelocity` (`self.ParentHitbox`) (+ _returnvalue_2 (* _returnvalue_2 (-0.025 -0.025 0.0))) false "None")
            (`PrimitiveComponent.SetPhysicsAngularVelocityInRadians` (`self.ParentHitbox`) (`KismetMathLibrary.ClampVectorSize` (+ _returnvalue (* _returnvalue (`self.RollDeceleration`))) -14.0 14.0) false "None")))))))

(event `self.ReceiveBeginPlay`
  ;[0.1036 0.2599 0.9948 0.5] Set Initial Speeds
  (set `self.RollAcceleration` (0.0 0.0 0.4))
  (set `self.RollDeceleration` (0.0 0.0 -0.2))
  ; Set Input Mapping Context
  (bind _asbp_player_controller (cast `/Game/Blueprints/BP_PlayerController` (`self.GetController`)))
  (message `EnhancedInputSubsystemInterface.AddMappingContext` (pcsubsystem `EnhancedInputLocalPlayerSubsystem` _asbp_player_controller) "/Game/Input/IMC_Rolling.IMC_Rolling" 0 (struct)))

(event `EnhancedInput|/Game/Input/InputActions/ScrewMovement/IA_RollForward`
  (params (ActionValue :type Boolean) (ElapsedSeconds :type "Float (double-precision)") (TriggeredSeconds :type "Float (double-precision)") (InputAction :type "InputAction Object Reference" :default "/Game/Input/InputActions/ScrewMovement/IA_RollForward.IA_RollForward"))
  ;[0.15 0.06625 0.1412 0.5] Input For Rolling
  ;;[0.2135 0.01335 0.01369 0.5] Forward + Backward
  (:`Triggered`
    (`PrimitiveComponent.SetPhysicsAngularVelocityInRadians` (`self.ParentHitbox`) (+ (`PrimitiveComponent.GetPhysicsAngularVelocityInRadians` (`self.ParentHitbox`) "None") (`self.ScaleByDeltaTime` (`KismetMathLibrary.TransformDirection` (`SceneComponent.GetRelativeTransform` (`self.ParentHitbox`)) (`self.RollAcceleration`)))) false "None"))
  (:`Started`
    (set `self.bIsRolling` true))
  (:`Canceled`
    (set `self.bIsRolling` false :!label _label)
    (`self.PrintAngularVelocity`))
  (:`Completed`
    (goto _label)))

(event `EnhancedInput|/Game/Input/InputActions/ScrewMovement/IA_WalkForward`
  (params (ActionValue :type Boolean) (ElapsedSeconds :type "Float (double-precision)") (TriggeredSeconds :type "Float (double-precision)") (InputAction :type "InputAction Object Reference" :default "/Game/Input/InputActions/ScrewMovement/IA_WalkForward.IA_WalkForward"))
  ;[0.1442 0.3646 0.3046 0.5] Input For Walking
  ;;[0.2135 0.01335 0.01369 0.5] Forward + Backward
  (:`Triggered`
    (`self.AddMovementInput` (50.0 0.0 0.0) 100.0))
  (:`Started`
    (`self.ActivateBounce` true))
  (:`Canceled`
    (`self.ActivateBounce` false :!label _label_2))
  (:`Completed`
    (goto _label_2)))

(event `ActivateBounce`
  (params (Activate :type Boolean))
  (bind (_relativelocation_x _relativelocation_y) (`KismetMathLibrary.BreakVector` (`SceneComponent.RelativeLocation` (`self.Cylinder`))))
  (bind (_relativelocation_x_2 _relativelocation_y_2) (`KismetMathLibrary.BreakVector` (`SceneComponent.RelativeLocation` (`self.Cylinder`))))
  ;[0.1496 0.7396 0 0.5] Bouncing Animation Event
  (if Activate
    (bind (_direction _height) (`Timeline|Timeline` :!via `PlayFromStart` :!label _label_3)
      (:`Update`
        (`SceneComponent.K2_SetRelativeLocation` (`self.Cylinder`) (`KismetMathLibrary.MakeVector` _relativelocation_x _relativelocation_y _height) false false))
      (:`Finished`
        (`SceneComponent.K2_SetRelativeLocation` (`self.Cylinder`) (`KismetMathLibrary.MakeVector` _relativelocation_x_2 _relativelocation_y_2) false false :!label _label_4)))
    (else
      (`|ExecutionSequence`
        (:`then_0`
          (goto _label_3 :!via `Stop`))
        (:`then_1`
          (goto _label_4))))))

(event `EnhancedInput|/Game/Input/InputActions/CameraMovement/IA_CameraRotation_X`
  (params (ActionValue :type "Float (double-precision)") (ElapsedSeconds :type "Float (double-precision)") (TriggeredSeconds :type "Float (double-precision)") (InputAction :type "InputAction Object Reference" :default "/Game/Input/InputActions/CameraMovement/IA_CameraRotation_X.IA_CameraRotation_X"))
  (bind (_returnvalue_roll _returnvalue_pitch _returnvalue_yaw) (`KismetMathLibrary.BreakRotator` (`SpringArmComponent.GetTargetRotation` (`self.SpringArm`))))
  ; Testing camera rotation
  (:`Triggered`
    (`SceneComponent.K2_SetRelativeRotation` (`self.SpringArm`) (`KismetMathLibrary.MakeRotator` _returnvalue_roll _returnvalue_pitch (+ _returnvalue_yaw ActionValue)) false false)))

(event `EnhancedInput|/Game/Input/InputActions/ScrewMovement/IA_WalkBackward`
  (params (ActionValue :type Boolean) (ElapsedSeconds :type "Float (double-precision)") (TriggeredSeconds :type "Float (double-precision)") (InputAction :type "InputAction Object Reference" :default "/Game/Input/InputActions/ScrewMovement/IA_WalkBackward.IA_WalkBackward"))
  ;[0.1442 0.3646 0.3046 0.5] Input For Walking
  ;;[0.2135 0.01335 0.01369 0.5] Forward + Backward
)

(event `EnhancedInput|/Game/Input/InputActions/CameraMovement/IA_CameraRotation_Y`
  (params (ActionValue :type "Float (double-precision)") (ElapsedSeconds :type "Float (double-precision)") (TriggeredSeconds :type "Float (double-precision)") (InputAction :type "InputAction Object Reference" :default "/Game/Input/InputActions/CameraMovement/IA_CameraRotation_Y.IA_CameraRotation_Y"))
  (bind (_returnvalue_roll _returnvalue_pitch _returnvalue_yaw) (`KismetMathLibrary.BreakRotator` (`SpringArmComponent.GetTargetRotation` (`self.SpringArm`))))
  ; Testing camera rotation
  (:`Triggered`
    (`SceneComponent.K2_SetRelativeRotation` (`self.SpringArm`) (`KismetMathLibrary.MakeRotator` _returnvalue_roll (`KismetMathLibrary.FClamp` (+ ActionValue _returnvalue_pitch) -75.0 -15.0) _returnvalue_yaw) false false)))

(event `EnhancedInput|/Game/Input/InputActions/ScrewMovement/IA_RollBackward`
  (params (ActionValue :type Boolean) (ElapsedSeconds :type "Float (double-precision)") (TriggeredSeconds :type "Float (double-precision)") (InputAction :type "InputAction Object Reference" :default "/Game/Input/InputActions/ScrewMovement/IA_RollBackward.IA_RollBackward"))
  ;[0.15 0.06625 0.1412 0.5] Input For Rolling
  ;;[0.2135 0.01335 0.01369 0.5] Forward + Backward
  (:`Triggered`
    (`PrimitiveComponent.SetPhysicsAngularVelocityInRadians` (`self.ParentHitbox`) (- (`PrimitiveComponent.GetPhysicsAngularVelocityInRadians` (`self.ParentHitbox`) "None") (`self.ScaleByDeltaTime` (`KismetMathLibrary.TransformDirection` (`SceneComponent.GetRelativeTransform` (`self.ParentHitbox`)) (`self.RollAcceleration`)))) false "None"))
  (:`Started`
    (set `self.bIsRolling` true))
  (:`Canceled`
    (set `self.bIsRolling` false :!label _label_5)
    (`self.PrintAngularVelocity`))
  (:`Completed`
    (goto _label_5)))

(event `EnhancedInput|/Game/Input/InputActions/ScrewMovement/IA_RollLeft`
  (params (ActionValue :type Boolean) (ElapsedSeconds :type "Float (double-precision)") (TriggeredSeconds :type "Float (double-precision)") (InputAction :type "InputAction Object Reference" :default "/Game/Input/InputActions/ScrewMovement/IA_RollLeft.IA_RollLeft"))
  (bind (_relativerotation_roll _relativerotation_pitch _relativerotation_yaw) (`KismetMathLibrary.BreakRotator` (`SceneComponent.RelativeRotation` (`self.ParentHitbox`))))
  (bind (_returnvalue_x _returnvalue_y) (`KismetMathLibrary.BreakVector` (`KismetMathLibrary.InverseTransformDirection` (`self.GetTransform`) (`PrimitiveComponent.GetPhysicsAngularVelocityInRadians` (`self.ParentHitbox`) "None"))))
  ;[0.15 0.06625 0.1412 0.5] Input For Rolling
  ;;[0.03737 0.2708 0.03669 0.5] Turning Based on Velocity
  (:`Triggered`
    (`SceneComponent.K2_SetRelativeRotation` (`self.ParentHitbox`) (`KismetMathLibrary.MakeRotator` _relativerotation_roll _relativerotation_pitch (- _relativerotation_yaw (+ (`KismetMathLibrary.Abs` (/ _returnvalue_x 25.0)) (`KismetMathLibrary.Abs` (/ _returnvalue_y 25.0))))) false false)))

(event `EnhancedInput|/Game/Input/InputActions/ScrewMovement/IA_WalkLeft`
  (params (ActionValue :type Boolean) (ElapsedSeconds :type "Float (double-precision)") (TriggeredSeconds :type "Float (double-precision)") (InputAction :type "InputAction Object Reference" :default "/Game/Input/InputActions/ScrewMovement/IA_WalkLeft.IA_WalkLeft"))
  ;[0.1442 0.3646 0.3046 0.5] Input For Walking
)

(event `EnhancedInput|/Game/Input/InputActions/ScrewMovement/IA_WalkRight`
  (params (ActionValue :type Boolean) (ElapsedSeconds :type "Float (double-precision)") (TriggeredSeconds :type "Float (double-precision)") (InputAction :type "InputAction Object Reference" :default "/Game/Input/InputActions/ScrewMovement/IA_WalkRight.IA_WalkRight"))
  ;[0.1442 0.3646 0.3046 0.5] Input For Walking
)

(event `EnhancedInput|/Game/Input/InputActions/ScrewMovement/IA_RollRight`
  (params (ActionValue :type Boolean) (ElapsedSeconds :type "Float (double-precision)") (TriggeredSeconds :type "Float (double-precision)") (InputAction :type "InputAction Object Reference" :default "/Game/Input/InputActions/ScrewMovement/IA_RollRight.IA_RollRight"))
  (bind (_relativerotation_roll _relativerotation_pitch _relativerotation_yaw) (`KismetMathLibrary.BreakRotator` (`SceneComponent.RelativeRotation` (`self.ParentHitbox`))))
  (bind (_returnvalue_x _returnvalue_y) (`KismetMathLibrary.BreakVector` (`KismetMathLibrary.InverseTransformDirection` (`self.GetTransform`) (`PrimitiveComponent.GetPhysicsAngularVelocityInRadians` (`self.ParentHitbox`) "None"))))
  ;[0.15 0.06625 0.1412 0.5] Input For Rolling
  ;;[0.03737 0.2708 0.03669 0.5] Turning Based on Velocity
  (:`Triggered`
    (`SceneComponent.K2_SetRelativeRotation` (`self.ParentHitbox`) (`KismetMathLibrary.MakeRotator` _relativerotation_roll _relativerotation_pitch (+ _relativerotation_yaw (`KismetMathLibrary.Abs` (/ _returnvalue_x 25.0)) (`KismetMathLibrary.Abs` (/ _returnvalue_y 25.0)))) false false)))

(event `EnhancedInput|/Game/Input/InputActions/ScrewMovement/IA_RollForward`
  (params (ActionValue :type Boolean) (ElapsedSeconds :type "Float (double-precision)") (TriggeredSeconds :type "Float (double-precision)") (InputAction :type "InputAction Object Reference" :default "/Game/Input/InputActions/ScrewMovement/IA_RollForward.IA_RollForward"))
  ;[0 0 0 0.687] Moving with Linear Velocity (Depreciated)
)

(event `EnhancedInput|/Game/Input/InputActions/ScrewMovement/IA_RollBackward`
  (params (ActionValue :type Boolean) (ElapsedSeconds :type "Float (double-precision)") (TriggeredSeconds :type "Float (double-precision)") (InputAction :type "InputAction Object Reference" :default "/Game/Input/InputActions/ScrewMovement/IA_RollBackward.IA_RollBackward"))
  ;[0 0 0 0.687] Moving with Linear Velocity (Depreciated)
)

(event `EnhancedInput|/Game/Input/InputActions/ScrewMovement/IA_SwitchModes`
  (params (ActionValue :type Boolean) (ElapsedSeconds :type "Float (double-precision)") (TriggeredSeconds :type "Float (double-precision)") (InputAction :type "InputAction Object Reference" :default "/Game/Input/InputActions/ScrewMovement/IA_SwitchModes.IA_SwitchModes"))
  ;[0.05556 0 0.8802 0.5] SWITCH MOVEMENT MODES
  (:`Started`
    (bind _asbp_player_controller (cast `/Game/Blueprints/BP_PlayerController` (`self.GetController`)))
    (bind _returnvalue (pcsubsystem `EnhancedInputLocalPlayerSubsystem` _asbp_player_controller))
    ;; If Rolling, then Walk
    (if (`.ReturnValue` (`EnhancedInputSubsystemInterface.HasMappingContext` _returnvalue "/Game/Input/IMC_Rolling.IMC_Rolling"))
      (`SceneComponent.K2_SetRelativeRotation` :`self` (`self.ParentHitbox`))
      (`PrimitiveComponent.SetCollisionEnabled` (`self.ParentHitbox`) "QueryAndPhysics")
      (`PrimitiveComponent.SetCollisionEnabled` (`self.Cylinder`) "QueryOnly")
      (`EnhancedInputSubsystemInterface.RemoveMappingContext` _returnvalue "/Game/Input/IMC_Rolling.IMC_Rolling" (struct))
      (`EnhancedInputSubsystemInterface.AddMappingContext` _returnvalue "/Game/Input/IMC_Walking.IMC_Walking" 0 (struct))
      (set `self.bIsWalking` true)
      (`KismetSystemLibrary.PrintString` "true")
      (`PrimitiveComponent.SetSimulatePhysics` (`self.ParentHitbox`) false)
      (else
        ;; If Walking, then Roll
        (if (`.ReturnValue` (`EnhancedInputSubsystemInterface.HasMappingContext` _returnvalue "/Game/Input/IMC_Walking.IMC_Walking"))
          (`SceneComponent.K2_SetRelativeRotation` (`self.ParentHitbox`) (struct :`Roll` 90.0) false false)
          (`PrimitiveComponent.SetCollisionEnabled` (`self.ParentHitbox`) "QueryAndPhysics")
          (`PrimitiveComponent.SetCollisionEnabled` (`self.Cylinder`) "QueryAndPhysics")
          (`EnhancedInputSubsystemInterface.RemoveMappingContext` _returnvalue "/Game/Input/IMC_Walking.IMC_Walking" (struct))
          (`EnhancedInputSubsystemInterface.AddMappingContext` _returnvalue "/Game/Input/IMC_Rolling.IMC_Rolling" 0 (struct))
          (set `self.bIsWalking` false)
          (`KismetSystemLibrary.PrintString` "false")
          (`PrimitiveComponent.SetSimulatePhysics` (`self.ParentHitbox`) true))))))

(fn `SetMovementDirections`
  (params (bIsWalking :type Boolean) (MovementDirection :type "/Game/Blueprints/ExtraData/MovementDirections Enum" :default "NewEnumerator0"))
  (`KismetArrayLibrary.Array_Set` (`self.bIsWalkingDirectionArray`) (`KismetMathLibrary.Conv_ByteToInt` MovementDirection) bIsWalking))

(fn `UserConstructionScript`)